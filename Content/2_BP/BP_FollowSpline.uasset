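; Spline follower actor that moves its ReferencePoint component along its Spline at a set Speed.
; After a fixed delay from BeginPlay, it enables movement and plays a Mario Kart stadium music track as 2D sound.
; Each Tick advances Distance and applies the spline's local location and rotation, preserving the component's scale.
; The IsLooping branch checks for the spline's end but does nothing, so Distance never wraps.
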(event `self.ReceiveBeginPlay`
  (`KismetSystemLibrary.Delay` 6.8)
  (set `self.Able2Move` true)
  (`GameplayStatics.SpawnSound2D` "/Game/5_FX/Audio/bgm_mariokart_stardium_.bgm_mariokart_stardium_" 1.0 1.0 0.0 null))

(event `self.ReceiveTick`
  (params (DeltaSeconds :type "Float (single-precision)"))
  (bind (_returnvalue_location _returnvalue_rotation) (`KismetMathLibrary.BreakTransform` (`SplineComponent.GetTransformAtDistanceAlongSpline` (`self.Spline`) (`self.Distance`) "Local" false)))
  (if (`self.Able2Move`)
    (set `self.Distance` (+ (* DeltaSeconds (`self.Speed`)) (`self.Distance`)))
    (`SceneComponent.K2_SetRelativeTransform` (`self.ReferencePoint`) (`KismetMathLibrary.MakeTransform` _returnvalue_location _returnvalue_rotation (`SceneComponent.RelativeScale3D` (`self.ReferencePoint`))) false false)
    (if (`self.isLooping`)
      (if (> (`self.Distance`) (`SplineComponent.GetSplineLength` (`self.Spline`)))
        _))))

(fn `UserConstructionScript`)