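; Player kart Blueprint that drives drift and dash effects and shows the opening countdown widget once.
; Tick reads the controller's drift flag and checks max walk speed, re-spawning socket-attached sparks or nitro every qualifying frame.
; An authority switch calls Server RPCs directly or through Client RPC wrappers named Multi.
; Dashing also pulses screen blur through a Material Parameter Collection; leftover timer nodes never run.
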(event `self.ReceiveTick`
  (params (DeltaSeconds :type "Float (single-precision)"))
  (bind _asmario_kart_player_controller (cast `MarioKartPlayerController` (`GameplayStatics.GetPlayerController` 0)))
  (if (`MarioKartPlayerController.bIsDriftkartBody` _asmario_kart_player_controller)
    (`/Engine/EditorBlueprintResources/ActorMacros.Switch Has Authority`
      (:`Authority`
        (`self.ServerDriftEffectOn`))
      (:`Remote`
        (`self.MultiDriftEffectOn`))))
  (if (>= (`CharacterMovementComponent.MaxWalkSpeed` (`self.CharacterMovement`)) 2000.0)
    (`/Engine/EditorBlueprintResources/ActorMacros.Switch Has Authority`
      (:`Authority`
        (`KismetSystemLibrary.PrintString` "Server")
        (`self.ServerDashEffectOn`)
        (`self.CameraEffect`))
      (:`Remote`
        (`KismetSystemLibrary.PrintString` "Client")
        (`self.MultiDashEffectOn`)
        (`self.CameraEffect`))))
  (`|ExecutionSequence`
    (:`then_0`
      (`/Engine/EditorBlueprintResources/StandardMacros.DoOnce` false
        (:`Completed`
          (bind _returnvalue (`|CreateWidget` "/Game/2_BP/UI/UI_CountDown.UI_CountDown_C" (`GameplayStatics.GetPlayerController` 0)))
          (`UserWidget.AddToViewport` _returnvalue 0)
          (`KismetSystemLibrary.Delay` 5.5)
          (`Widget.RemoveFromParent` _returnvalue))))))

(event `ServerDriftEffectOn`
  (bind _kartwheelcomp (`self.kartwheelComp`))
  ;[1 1 1] Server RPC - DriftEffect
  (`GameplayStatics.SpawnEmitterAttached` "/Game/5_FX/P_Sparks1.P_Sparks1" _kartwheelcomp "DriftEffect_L" (`SceneComponent.GetSocketLocation` _kartwheelcomp "DriftEffect_L") (struct) (1.0 1.0 1.0) "KeepWorldPosition")
  (`GameplayStatics.SpawnEmitterAttached` "/Game/5_FX/P_Sparks1.P_Sparks1" _kartwheelcomp "DriftEffect_R" (`SceneComponent.GetSocketLocation` _kartwheelcomp "DriftEffect_R") (struct) (1.0 1.0 1.0) "KeepWorldPosition"))

(event `ServerDashEffectOn`
  (bind _kartmeshcomp (`self.kartmeshComp`))
  (bind _kartmeshcomp_2 (`self.kartmeshComp`))
  ;[1 1 1] Server RPC
  (`NiagaraFunctionLibrary.SpawnSystemAttached` "/Game/5_FX/Art/Boost/FX_Nitro.FX_Nitro" _kartmeshcomp_2 "FX_Dash_L" (`SceneComponent.GetSocketLocation` _kartmeshcomp_2 "FX_Dash_L") (struct) "KeepWorldPosition" true)
  (`NiagaraFunctionLibrary.SpawnSystemAttached` "/Game/5_FX/Art/Boost/FX_Nitro.FX_Nitro" _kartmeshcomp "FX_Dash_R" (`SceneComponent.GetSocketLocation` _kartmeshcomp "FX_Dash_R") (struct) "KeepWorldPosition" true))

(event `MultiDriftEffectOn`
  ;[1 1 1] Client RPC - DriftEffect
  (`self.ServerDriftEffectOn`))

(event `MultiDashEffectOn`
  ;[1 1 1] Client RPC
  (`self.ServerDashEffectOn`))

(event `CameraEffect`
  ;[1 1 1] camera effect
  (`KismetMaterialLibrary.SetScalarParameterValue` "/Game/5_FX/PC_CameraEffect.PC_CameraEffect" "Blur" 1.0)
  (`KismetSystemLibrary.Delay` 0.8)
  (`KismetMaterialLibrary.SetScalarParameterValue` "/Game/5_FX/PC_CameraEffect.PC_CameraEffect" "Blur"))

(fn `UserConstructionScript`)