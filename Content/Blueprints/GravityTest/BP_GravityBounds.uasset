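; BP_GravityBounds is a spherical gravity zone that sets the gravity of KartNinja actors inside it using its own location.
; A non-looping timer started on BeginPlay runs the update once, 0.01 seconds later, so gravity is not refreshed afterward.
; The update loops over all KartNinja actors, tests squared distance against the Bounds sphere radius, and passes the zone's location to SetGravity on those inside.
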(event `self.ReceiveBeginPlay`
  (`KismetSystemLibrary.K2_SetTimerDelegate` (delegate `UpdateGravity`) 0.01))

(event `UpdateGravity`
  (`self.SetPlayersGravity`))

(fn `IsInsideBounds`
  (params (Actor :type "Actor Object Reference"))
  (returns (`IsInsideBounds?` :type Boolean))
  (bind (_returnvalue_x _returnvalue_y _returnvalue_z) (`KismetMathLibrary.BreakVector` (`self.K2_GetActorLocation`)))
  (bind (_returnvalue_x_2 _returnvalue_y_2 _returnvalue_z_2) (`KismetMathLibrary.BreakVector` (`self.K2_GetActorLocation` Actor)))
  (return (< (+ (`KismetMathLibrary.Square` (- _returnvalue_x_2 _returnvalue_x)) (`KismetMathLibrary.Square` (- _returnvalue_y_2 _returnvalue_y)) (`KismetMathLibrary.Square` (- _returnvalue_z_2 _returnvalue_z))) (`KismetMathLibrary.Square` (`SphereComponent.SphereRadius` (`self.Bounds`))))))

(fn `SetPlayersGravity`
  (bind _outactors (`GameplayStatics.GetAllActorsOfClass` "/Game/Blueprints/GravityTest/KartNinja.KartNinja_C"))
  (for _array_element _outactors
    (if (`self.IsInsideBounds` _array_element)
      (`/Game/Blueprints/GravityTest/KartNinja.SetGravity` _array_element (`self.K2_GetActorLocation`)))))

(fn `UserConstructionScript`)