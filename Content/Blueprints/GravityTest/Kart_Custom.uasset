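; Player-driven kart in a gravity test that accelerates with an input and steers by turning controller yaw with the horizontal axis.
; Each tick, MoveVertical lerps CurrentSpeed toward forward max, a negative reverse target or zero, and prints it.
; Movement input crosses control right with capsule up, so direction follows the capsule's tilt.
; That input is applied only while accelerating, so reverse and slowdown only change the speed value.
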(event `InputAction|Acc`
  (params (Key :type "Key Structure"))
  (:`Pressed`
    (set `self.IsAccel` true))
  (:`Released`
    (set `self.IsAccel` false)))

(event `InputAction|MoveBack`
  (params (Key :type "Key Structure"))
  (:`Pressed`
    (set `self.IsBackMoving` true))
  (:`Released`
    (set `self.IsBackMoving` false)))

(event `InputAxis|Horizontal`
  (params (AxisValue :type "Float (single-precision)"))
  (bind _output_get (set `self.HorizontalValue` AxisValue))
  (`self.AddControllerYawInput` _output_get))

(event `self.ReceiveTick`
  (params (DeltaSeconds :type "Float (single-precision)"))
  (`self.MoveVertical`)
  (if (`self.IsAccel`)
    (`self.AddMovementInput` (`KismetMathLibrary.Normal` (`KismetMathLibrary.Cross_VectorVector` (`KismetMathLibrary.GetRightVector` (`self.GetControlRotation`)) (`KismetMathLibrary.GetUpVector` (`SceneComponent.K2_GetComponentRotation` (`self.CapsuleComponent`))))) (`self.CurrentSpeed`))))

(fn `MoveVertical`
  (if (or (`self.IsAccel`) (`self.IsBackMoving`))
    (if (`self.IsAccel`)
      ;[1 1 1] 전진 가속 (Alpha 값 수정으로 가속 변화 가능)
      (bind _output_get (set `self.CurrentSpeed` (`KismetMathLibrary.Lerp` (`self.CurrentSpeed`) (`self.MaxSpeed`) (* (`GameplayStatics.GetWorldDeltaSeconds`) 1.5))))
      (`KismetSystemLibrary.PrintString` (`KismetStringLibrary.Conv_DoubleToString` _output_get) true true (struct :`R` 0.564706 :`G` 1.0 :`B` 0.396078 :`A` 1.0) (`self.PrintTime`))
      (else
        ;[1 1 1] 후진 (가속 없음)
        (bind _output_get_2 (set `self.CurrentSpeed` (`KismetMathLibrary.Lerp` (`self.CurrentSpeed`) (* (`self.MaxSpeed`) -1.8) (`GameplayStatics.GetWorldDeltaSeconds`))))
        (`KismetSystemLibrary.PrintString` (`KismetStringLibrary.Conv_DoubleToString` _output_get_2) true true (struct :`R` 0.564706 :`G` 1.0 :`B` 0.396078 :`A` 1.0) (`self.PrintTime`))))
    (else
      ;[1 1 1] 속도를 0으로 조정
      (bind _output_get_3 (set `self.CurrentSpeed` (`KismetMathLibrary.Lerp` (`self.CurrentSpeed`) 0.0 (* (`GameplayStatics.GetWorldDeltaSeconds`) 3.0))))
      (`KismetSystemLibrary.PrintString` (`KismetStringLibrary.Conv_DoubleToString` _output_get_3) true true (struct :`R` 0.564706 :`G` 1.0 :`B` 0.396078 :`A` 1.0) (`self.PrintTime`)))))

(fn `UserConstructionScript`)