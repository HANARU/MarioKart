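; Test kart character built on Ninja Character movement, combining kart-style speed control with point gravity.
; MoveVertical eases CurrentSpeed by delta-time-scaled Lerp toward forward max, a negative reverse target or zero, based on IsAccel and IsMovingBack.
; SetGravity casts CharacterMovement to NinjaCharacterMovementComponent and points gravity at a given center.
; These functions and CheckInput print debug values; none is called or applies speed to movement here.
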(fn `CheckInput`
  (`KismetSystemLibrary.PrintString` (`KismetStringLibrary.Concat_StrStr` "Value : " (`KismetStringLibrary.Conv_DoubleToString` (`self.HorizontalValue`)) " Accel : " (`KismetStringLibrary.Conv_BoolToString` (`self.IsAccel`))) true true (struct :`G` 0.66 :`B` 1.0 :`A` 1.0) (`self.PrintTime`)))

(fn `MoveVertical`
  (if (or (`self.IsAccel`) (`self.IsMovingBack`))
    (if (`self.IsAccel`)
      ;[1 1 1] 전진 가속 (Alpha 값 수정으로 가속 변화 가능)
      (set `self.Alpha` (* (`GameplayStatics.GetWorldDeltaSeconds`) 1.5))
      (bind _output_get (set `self.CurrentSpeed` (`KismetMathLibrary.Lerp` (`self.CurrentSpeed`) (`self.MaxSpeed`) (`self.Alpha`))))
      (`KismetSystemLibrary.PrintString` (`KismetStringLibrary.Conv_DoubleToString` _output_get) true true (struct :`R` 0.564706 :`G` 1.0 :`B` 0.396078 :`A` 1.0) (`self.PrintTime`))
      (else
        ;[1 1 1] 후진 (가속 없음)
        (bind _output_get_2 (set `self.CurrentSpeed` (`KismetMathLibrary.Lerp` (`self.CurrentSpeed`) (* (`self.MaxSpeed`) -1.8) (`GameplayStatics.GetWorldDeltaSeconds`))))
        (`KismetSystemLibrary.PrintString` (`KismetStringLibrary.Conv_DoubleToString` _output_get_2) true true (struct :`R` 0.564706 :`G` 1.0 :`B` 0.396078 :`A` 1.0) (`self.PrintTime`))))
    (else
      ;[1 1 1] 속도를 0으로 조정
      (bind _output_get_3 (set `self.CurrentSpeed` (`KismetMathLibrary.Lerp` (`self.CurrentSpeed`) 0.0 (* (`GameplayStatics.GetWorldDeltaSeconds`) 3.0))))
      (`KismetSystemLibrary.PrintString` (`KismetStringLibrary.Conv_DoubleToString` _output_get_3) true true (struct :`R` 0.564706 :`G` 1.0 :`B` 0.396078 :`A` 1.0) (`self.PrintTime`)))))

(fn `SetGravity`
  (params (`Center of Gravity` :type "Vector Structure"))
  (bind _asninja_character_movement_component (cast `NinjaCharacterMovementComponent` (`self.CharacterMovement`)))
  (`NinjaCharacterMovementComponent.SetPointGravityDirection` _asninja_character_movement_component `Center of Gravity`)
  (`KismetSystemLibrary.PrintString` (`KismetStringLibrary.Conv_VectorToString` `Center of Gravity`) true true (struct :`R` 0.807059 :`G` 1.0 :`B` 0.047971 :`A` 1.0) (`self.PrintTime`)))

(fn `UserConstructionScript`)