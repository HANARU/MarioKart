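; Kart-style test character with acceleration, reverse and point gravity through the Ninja character movement component.
; Tick eases CurrentSpeed toward forward, reverse or zero targets in MoveVertical, then applies it as forward movement input only while steering is idle.
; Horizontal input adds sideways movement while speed is positive.
; Turning is unfinished: yaw input is computed but the rotation nodes are disconnected, and debug prints run throughout.
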(event `InputAxis|horizontal`
  (params (AxisValue :type "Float (single-precision)"))
  (set `self.HorizontalValue` AxisValue)
  (if (> (`self.CurrentSpeed`) 0.0)
    (set `self.HorizontalRotation` (+ AxisValue (`self.HorizontalRotation`)))
    (`self.AddMovementInput` (`KismetMathLibrary.GetRightVector` (`KismetMathLibrary.MakeRotator` 0.0)) AxisValue)))

(event `InputAction|Acc`
  (params (Key :type "Key Structure"))
  (:`Pressed`
    (set `self.IsAccel` true))
  (:`Released`
    (set `self.IsAccel` false)))

(event `InputAction|MoveBack`
  (params (Key :type "Key Structure"))
  (:`Pressed`
    (set `self.IsMovingBack` true))
  (:`Released`
    (set `self.IsMovingBack` false)))

(event `self.ReceiveTick`
  (params (DeltaSeconds :type "Float (single-precision)"))
  (`KismetSystemLibrary.PrintString` (`KismetStringLibrary.Conv_DoubleToString` (`self.CurrentSpeed`)) true true (struct :`G` 0.66 :`B` 1.0 :`A` 1.0) (`self.PrintTime`))
  (`KismetSystemLibrary.PrintString` (`KismetStringLibrary.Conv_RotatorToString` (`self.K2_GetActorRotation`)) true true (struct :`G` 0.66 :`B` 1.0 :`A` 1.0) (`self.PrintTime`))
  (`|ExecutionSequence`
    (:`then_0`
      (`self.MoveVertical`))
    (:`then_1`
      (if (== (`self.HorizontalValue`) 0.0)
        (`self.AddMovementInput` (`self.GetActorForwardVector`) (`self.CurrentSpeed`))
        (`KismetSystemLibrary.PrintString` (`KismetStringLibrary.Concat_StrStr` "Rot Value : " (`KismetStringLibrary.Conv_DoubleToString` (* DeltaSeconds (`self.HorizontalRotation`)))) true true (struct :`R` 1.0 :`G` 0.138485 :`B` 0.058804 :`A` 1.0) (`self.PrintTime`))))
    (:`then_2`
      ;[1 1 1] 좌우 회전 구현 (반드시 수정 필요)
      (if (!= (`self.HorizontalValue`) 0.0)
        (bind _output_get (set `self.YawInputValue` (* (`self.HorizontalValue`) (`self.BaseTurnRate`) (`GameplayStatics.GetWorldDeltaSeconds`))))))))

(fn `CheckInput`
  (`KismetSystemLibrary.PrintString` (`KismetStringLibrary.Concat_StrStr` "Value : " (`KismetStringLibrary.Conv_DoubleToString` (`self.HorizontalValue`)) " Accel : " (`KismetStringLibrary.Conv_BoolToString` (`self.IsAccel`))) true true (struct :`G` 0.66 :`B` 1.0 :`A` 1.0) (`self.PrintTime`)))

(fn `MoveVertical`
  (if (or (`self.IsAccel`) (`self.IsMovingBack`))
    (if (`self.IsAccel`)
      ;[1 1 1] 전진 가속 (Alpha 값 수정으로 가속 변화 가능)
      (bind _output_get (set `self.CurrentSpeed` (`KismetMathLibrary.Lerp` (`self.CurrentSpeed`) (`self.MaxSpeed`) (* (`GameplayStatics.GetWorldDeltaSeconds`) 1.5))))
      (`KismetSystemLibrary.PrintString` (`KismetStringLibrary.Conv_DoubleToString` _output_get) true true (struct :`G` 0.66 :`B` 1.0 :`A` 1.0) (`self.PrintTime`))
      (else
        ;[1 1 1] 후진 (가속 없음)
        (bind _output_get_2 (set `self.CurrentSpeed` (`KismetMathLibrary.Lerp` (`self.CurrentSpeed`) (* (`self.MaxSpeed`) -1.8) (`GameplayStatics.GetWorldDeltaSeconds`))))
        (`KismetSystemLibrary.PrintString` (`KismetStringLibrary.Conv_DoubleToString` _output_get_2) true true (struct :`G` 0.66 :`B` 1.0 :`A` 1.0) (`self.PrintTime`))))
    (else
      ;[1 1 1] Comment
      (bind _output_get_3 (set `self.CurrentSpeed` (`KismetMathLibrary.Lerp` (`self.CurrentSpeed`) 0.0 (* (`GameplayStatics.GetWorldDeltaSeconds`) 3.0))))
      (`KismetSystemLibrary.PrintString` (`KismetStringLibrary.Conv_DoubleToString` _output_get_3) true true (struct :`G` 0.66 :`B` 1.0 :`A` 1.0) (`self.PrintTime`)))))

(fn `SetGravity`
  (params (`Center of Gravity` :type "Vector Structure"))
  (bind _asninja_character_movement_component (cast `NinjaCharacterMovementComponent` (`self.CharacterMovement`)))
  (`NinjaCharacterMovementComponent.SetPointGravityDirection` _asninja_character_movement_component `Center of Gravity`)
  (`KismetSystemLibrary.PrintString` (`KismetStringLibrary.Conv_VectorToString` `Center of Gravity`) true true (struct :`R` 0.807059 :`G` 1.0 :`B` 0.047971 :`A` 1.0) (`self.PrintTime`)))

(fn `UserConstructionScript`)