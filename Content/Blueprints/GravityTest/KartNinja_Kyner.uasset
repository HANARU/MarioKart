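; Player-driven kart character prototype with acceleration, reverse, drifting and point gravity through NinjaCharacterMovementComponent.
; Tick calls MoveVertical to lerp CurrentSpeed toward forward, reverse or zero, then scales movement input along collapsed-graph directions.
; The horizontal axis drives controller yaw; holding accelerate and jump accumulates DriftTime, changing turn rate and temporarily boosting MaxWalkSpeed before a delayed reset.
; SetGravity sets the gravity point; debug prints run throughout.
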(event `self.ReceiveBeginPlay`
  (set `self.StartRotation` (`SceneComponent.K2_GetComponentRotation` (`self.KartBody`))))

(event `InputAxis|horizontal`
  (params (AxisValue :type "Float (single-precision)"))
  (bind _output_get (set `self.HorizontalValue` AxisValue))
  (if (!= _output_get 0.0)
    (if (`self.IsMovingBack`)
      ;[1 1 1] 후진
      (`self.AddControllerYawInput` (`KismetMathLibrary.Lerp` _output_get 0.0 0.3)))
    ;[1 1 1] 엑셀키 눌렀을 때
    (if (`self.IsAccel`)
      ;[1 1 1] 점프키 눌렀을 때
      (if (`self.IsJump`)
        ;[1 1 1] 엑셀키, 점프키 둘 다 눌렀을 때 회전율  더 높게 설정
        (`self.AddControllerYawInput` (`KismetMathLibrary.Lerp` 0.0 _output_get 0.7))
        (`KismetSystemLibrary.PrintString` "Driftstart" true true (struct :`G` 0.66 :`B` 1.0 :`A` 1.0) (`self.PrintTime`))
        (if (> (`self.DriftTime`) 6.0)
          ;[1 1 1] 기본 회전율
          (`self.AddControllerYawInput` (`KismetMathLibrary.Lerp` 0.0 (`self.HorizontalValue`) 0.3))
          (`KismetSystemLibrary.PrintString` "DriftEnd" true true (struct :`G` 0.66 :`B` 1.0 :`A` 1.0) (`self.PrintTime`))
          ;[1 1 1] 드리프트 타임, 최고 속도 리셋
          (set `self.DriftTime` 0.0)
          (set `CharacterMovementComponent.MaxWalkSpeed` 600.0 (`self.CharacterMovement`))
          (else
            ;[1 1 1] 드리프트 회전율
            (`self.AddControllerYawInput` (`KismetMathLibrary.Lerp` 0.0 0.5 0.01))
            (`KismetSystemLibrary.PrintString` "Drift" true true (struct :`G` 0.66 :`B` 1.0 :`A` 1.0) (`self.PrintTime`))))
        (else
          ;[1 1 1] 기본 회전율
          (`self.AddControllerYawInput` (`KismetMathLibrary.Lerp` 0.0 _output_get 0.3))
          (`KismetSystemLibrary.PrintString` "No" true true (struct :`G` 0.66 :`B` 1.0 :`A` 1.0) (`self.PrintTime`)))))))

(event `InputAction|Acc`
  (params (Key :type "Key Structure"))
  (:`Pressed`
    (set `self.IsAccel` true))
  (:`Released`
    (set `self.IsAccel` false)))

(event `InputAction|MoveBack`
  (params (Key :type "Key Structure"))
  (:`Pressed`
    (set `self.IsMovingBack` true))
  (:`Released`
    (set `self.IsMovingBack` false)))

(event `InputAction|Jump`
  (params (Key :type "Key Structure"))
  ;[1 1 1] 점프키 눌렀을 때
  (:`Pressed`
    (set `self.IsJump` true))
  (:`Released`
    (set `self.IsJump` false)))

(event `self.ReceiveTick`
  (params (DeltaSeconds :type "Float (single-precision)"))
  (bind _returnvalue (`KismetMathLibrary.Normal` (`KismetMathLibrary.Cross_VectorVector` (`KismetMathLibrary.GetRightVector` (`self.GetControlRotation`)) (`KismetMathLibrary.GetUpVector` (`SceneComponent.K2_GetComponentRotation` (`self.KartBody`))))))
  (bind _returnvalue_2 (`KismetMathLibrary.Normal` (`KismetMathLibrary.Cross_VectorVector` (`KismetMathLibrary.GetRightVector` (`self.GetControlRotation`)) (`KismetMathLibrary.GetUpVector` (`SceneComponent.K2_GetComponentRotation` (`self.KartBody`))))))
  (`KismetSystemLibrary.PrintString` (`KismetStringLibrary.Conv_RotatorToString` (`self.K2_GetActorRotation`)) true true (struct :`R` 0.070746 :`B` 1.0 :`A` 1.0) (`self.PrintTime`))
  (`self.MoveVertical`)
  (if (`self.IsMovingBack`)
    ;[1 1 1] 후진할 때 이동
    (`KismetSystemLibrary.PrintString` "Hello" true true (struct :`G` 0.66 :`B` 1.0 :`A` 1.0) (`self.PrintTime`))
    (`self.AddMovementInput` (`KismetMathLibrary.Normal` (`KismetMathLibrary.Cross_VectorVector` (`KismetMathLibrary.GetRightVector` (`self.GetControlRotation`)) (`KismetMathLibrary.GetUpVector` (`SceneComponent.K2_GetComponentRotation` (`self.KartBody`))))) (`self.CurrentSpeed`))
    (else
      ;[1 1 1] 엑셀키 눌렀을 때
      (if (`self.IsAccel`)
        ;[1 1 1] 점프키 눌렀을 때
        (if (`self.IsJump`)
          ;[1 1 1] 드리프트 시간 누적
          (bind _output_get (set `self.DriftTime` (+ DeltaSeconds (`self.DriftTime`))))
          (`KismetSystemLibrary.PrintString` (`KismetStringLibrary.Conv_DoubleToString` _output_get) true true (struct :`G` 0.66 :`B` 1.0 :`A` 1.0) (`self.PrintTime`))
          ;[1 1 1] 드리프트 시간 2second
          (if (> (`self.DriftTime`) 1.0)
            ;[1 1 1] 드리프트 안 풀리게
            (set `self.IsJump` true)
            (set `self.IsAccel` true)
            ;[1 1 1] MaxWalkSpeed로 속도 바꾸기
            (set `CharacterMovementComponent.MaxWalkSpeed` 1500.0 (`self.CharacterMovement`))
            ;[1 1 1] 드리프트 시간동안 앞으로 빠르게 전진
            (`self.AddMovementInput` (`KismetMathLibrary.Normal` (`KismetMathLibrary.Cross_VectorVector` (`KismetMathLibrary.GetRightVector` (`self.GetControlRotation`)) (`KismetMathLibrary.GetUpVector` (`SceneComponent.K2_GetComponentRotation` (`self.KartBody`))))) (`self.CurrentSpeed`))
            ;[1 1 1] 드리프트 2초 지나고 기본으로 리셋
            (`KismetSystemLibrary.Delay` 2.0)
            ;[1 1 1] 드리프트 끝, 원래 움직임으로 돌아가고 드리프트 시간 리셋
            (set `CharacterMovementComponent.MaxWalkSpeed` 600.0 (`self.CharacterMovement`))
            (`KismetSystemLibrary.PrintString` "DriftEnd" true true (struct :`G` 0.66 :`B` 1.0 :`A` 1.0) (`self.PrintTime`))
            (set `self.IsJump` false)
            (set `self.IsDrift` false)
            (`self.AddMovementInput` (`KismetMathLibrary.Normal` (`KismetMathLibrary.Cross_VectorVector` (`KismetMathLibrary.GetRightVector` (`self.GetControlRotation`)) (`KismetMathLibrary.GetUpVector` (`SceneComponent.K2_GetComponentRotation` (`self.KartBody`))))) (`self.CurrentSpeed`))
            (set `self.DriftTime` 0.0)
            (else
              ;[1 1 1] 기본 이동
              (`KismetSystemLibrary.PrintString` (`KismetStringLibrary.Conv_VectorToString` _returnvalue))
              (`self.AddMovementInput` _returnvalue (`self.CurrentSpeed`))))
          (else
            (`KismetSystemLibrary.PrintString` (`KismetStringLibrary.Conv_VectorToString` _returnvalue_2) true true (struct :`R` 0.637701 :`G` 1.0 :`B` 0.487953 :`A` 1.0) (`self.PrintTime`))
            (`self.AddMovementInput` _returnvalue_2 (`self.CurrentSpeed`))))
        (else
          ;[1 1 1] 가속키 누르지 않을 때 서서히 감속
          (`self.AddMovementInput` (`KismetMathLibrary.Normal` (`KismetMathLibrary.Cross_VectorVector` (`KismetMathLibrary.GetRightVector` (`self.GetControlRotation`)) (`KismetMathLibrary.GetUpVector` (`SceneComponent.K2_GetComponentRotation` (`self.KartBody`))))) (`self.CurrentSpeed`)))))))

(fn `CheckInput`
  (`KismetSystemLibrary.PrintString` (`KismetStringLibrary.Concat_StrStr` "Value : " (`KismetStringLibrary.Conv_DoubleToString` (`self.HorizontalValue`)) " Accel : " (`KismetStringLibrary.Conv_BoolToString` (`self.IsAccel`))) true true (struct :`G` 0.66 :`B` 1.0 :`A` 1.0) (`self.PrintTime`)))

(fn `MoveVertical`
  (if (or (`self.IsAccel`) (`self.IsMovingBack`))
    (if (`self.IsAccel`)
      ;[1 1 1] 전진 가속 (Alpha 값 수정으로 가속 변화 가능)
      (set `self.Alpha` (* (`GameplayStatics.GetWorldDeltaSeconds`) 1.5))
      (bind _output_get (set `self.CurrentSpeed` (`KismetMathLibrary.Lerp` (`self.CurrentSpeed`) (`self.MaxSpeed`) (`self.Alpha`))))
      (`KismetSystemLibrary.PrintString` (`KismetStringLibrary.Conv_DoubleToString` _output_get) true true (struct :`R` 0.564706 :`G` 1.0 :`B` 0.396078 :`A` 1.0) (`self.PrintTime`))
      (else
        ;[1 1 1] 후진 (가속 없음)
        (bind _output_get_2 (set `self.CurrentSpeed` (`KismetMathLibrary.Lerp` (`self.CurrentSpeed`) (* (`self.MaxSpeed`) -1.8) (`GameplayStatics.GetWorldDeltaSeconds`))))
        (`KismetSystemLibrary.PrintString` (`KismetStringLibrary.Conv_DoubleToString` _output_get_2) true true (struct :`R` 0.564706 :`G` 1.0 :`B` 0.396078 :`A` 1.0) (`self.PrintTime`))))
    (else
      ;[1 1 1] 속도를 0으로 조정
      (bind _output_get_3 (set `self.CurrentSpeed` (`KismetMathLibrary.Lerp` (`self.CurrentSpeed`) 0.0 (* (`GameplayStatics.GetWorldDeltaSeconds`) 3.0))))
      (`KismetSystemLibrary.PrintString` (`KismetStringLibrary.Conv_DoubleToString` _output_get_3) true true (struct :`R` 0.564706 :`G` 1.0 :`B` 0.396078 :`A` 1.0) (`self.PrintTime`)))))

(fn `SetGravity`
  (params (`Center of Gravity` :type "Vector Structure"))
  (bind _asninja_character_movement_component (cast `NinjaCharacterMovementComponent` (`self.CharacterMovement`)))
  (`NinjaCharacterMovementComponent.SetPointGravityDirection` _asninja_character_movement_component `Center of Gravity`)
  (`KismetSystemLibrary.PrintString` (`KismetStringLibrary.Conv_VectorToString` `Center of Gravity`) true true (struct :`R` 0.807059 :`G` 1.0 :`B` 0.047971 :`A` 1.0) (`self.PrintTime`)))

(fn `UserConstructionScript`)